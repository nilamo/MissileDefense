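; Player projectile Blueprint that flies from its spawn point to a Destination and destroys what it reaches.
; Launch sets the timeline play rate from the inverse 2D distance, aiming for constant travel speed regardless of range.
; The timeline lerps the actor's location without sweeping.
; When it finishes, every other actor overlapping the CollisionRadius component is destroyed, then the projectile destroys itself.
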(event `Launch`
  (bind _returnvalue (`self.K2_GetActorLocation`))
  (set `self.StartLocation` _returnvalue)
  (`TimelineComponent.SetPlayRate` (`self.Timeline_0`) (* (/ 1.0 (`KismetMathLibrary.Vector_Distance2D` (`self.Destination`) _returnvalue)) 300.0))
  (bind (_direction _duration) (`Timeline|Timeline_0`)
    (:`Update`
      (`self.K2_SetActorLocation` (`KismetMathLibrary.VLerp` (`self.StartLocation`) (`self.Destination`) _duration)))
    (:`Finished`
      (for _array_element (`PrimitiveComponent.GetOverlappingActors` (`self.CollisionRadius`) null)
        (if (not (== _array_element self))
          (`self.K2_DestroyActor` _array_element)))
      (`self.K2_DestroyActor`))))

(fn `UserConstructionScript`)