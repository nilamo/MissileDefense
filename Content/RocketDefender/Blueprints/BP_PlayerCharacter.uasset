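; Player character for Rocket Defender that resolves mouse clicks to a tower.
; BeginPlay caches all BP_Tower actors in LivingTowers, and each Click press passes the cursor's visibility trace location to GetClosestTowerToTarget.
; That function compares each tower's 2D distance to the target against the character's own distance, rather than the current best, so the last qualifying tower wins.
; The click handler leaves the returned tower unused.
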(event `self.ReceiveBeginPlay`
  (bind _outactors (`GameplayStatics.GetAllActorsOfClass` "/Game/RocketDefender/Player/BP_Tower.BP_Tower_C"))
  (set `self.LivingTowers` _outactors))

(event `InputAction|Click`
  (params (Key :type "Key Structure"))
  (:`Pressed`
    (`self.GetClosestTowerToTarget` (`.Location` (`GameplayStatics.BreakHitResult` (`self.GetHitResultUnderCursorByChannel` "TraceTypeQuery1"))))))

(fn `GetClosestTowerToTarget`
  (params (Target :type "Vector Structure"))
  (returns (ClosestTower :type "/Game/RocketDefender/Player/BP_Tower Object Reference"))
  (locals (FoundTower :type "/Game/RocketDefender/Player/BP_Tower Object Reference"))
  (bind _livingtowers (`self.LivingTowers`))
  (set `local.FoundTower` (`|GetArrayItem` _livingtowers))
  (for _array_element _livingtowers
    (if (<= (`KismetMathLibrary.Vector_Distance2D` (`self.K2_GetActorLocation` _array_element) Target) (`KismetMathLibrary.Vector_Distance2D` (`self.K2_GetActorLocation`) Target))
      (set `local.FoundTower` _array_element)))
  (return (`local.FoundTower`)))

(fn `UserConstructionScript`)