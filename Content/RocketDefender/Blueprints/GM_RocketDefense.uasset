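; Game mode for Rocket Defender that escalates meteor attacks and tracks the population being defended.
; From BeginPlay, an endless loop adds a meteor generator, waits in proportion to Difficulty, then raises Difficulty, so generators accumulate at growing intervals.
; Each generator gets its source and destination boxes from pairs of actors tagged StartPoint and EndPoint.
; TakeDamage subtracts from Population, clamped at zero.
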(event `self.ReceiveBeginPlay`
  (`self.SpawnEnemySpawner` :!label _label)
  (`KismetSystemLibrary.Delay` (`KismetMathLibrary.Conv_IntToDouble` (* (`self.Difficulty`) 5)))
  (`/Engine/EditorBlueprintResources/StandardMacros.IncrementInt` (`self.Difficulty`)
    (:`  `
      (goto _label))))

(fn `SpawnEnemySpawner`
  (bind _returnvalue (`|SpawnActorFromClass` "/Game/RocketDefender/AI/BP_MeteorGenerator.BP_MeteorGenerator_C" (`KismetMathLibrary.MakeTransform` (0.0 0.0 0.0)) "Undefined" "OverrideRootScale" null null))
  (bind _outactors (`GameplayStatics.GetAllActorsWithTag` "StartPoint"))
  (set `/Game/RocketDefender/AI/BP_MeteorGenerator.SourceBox` (make `Box` (`self.K2_GetActorLocation` (`|GetArrayItem` _outactors)) (`self.K2_GetActorLocation` (`|GetArrayItem` _outactors 1))) _returnvalue)
  (bind _outactors_2 (`GameplayStatics.GetAllActorsWithTag` "EndPoint"))
  (set `/Game/RocketDefender/AI/BP_MeteorGenerator.DestinationBox` (make `Box` (`self.K2_GetActorLocation` (`|GetArrayItem` _outactors_2)) (`self.K2_GetActorLocation` (`|GetArrayItem` _outactors_2 1))) _returnvalue))

(fn `TakeDamage`
  (params (Damage :type Integer))
  (bind _population (`self.Population`))
  (set `self.Population` (`KismetMathLibrary.Clamp` (- _population Damage) 0 _population)))

(fn `UserConstructionScript`)