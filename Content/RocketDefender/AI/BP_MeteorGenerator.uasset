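; BP_MeteorGenerator periodically spawns meteors in Rocket Defender, sending each from a random source point toward a random destination.
; Tick accumulates time until a randomly varied delay passes, then spawns a BP_Meteor, sets its Destination and rerolls the delay.
; Random points use each box's Min as origin and full size as extent, so they range beyond SourceBox and DestinationBox.
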(event `self.ReceiveTick`
  (params (DeltaSeconds :type "Float (single-precision)"))
  (bind _should_spawn (`self.ShouldSpawnMeteor` DeltaSeconds))
  (if _should_spawn
    (`self.SpawnMeteor`)
    (`self.SetNextSpawnTime`)))

(fn `SetNextSpawnTime`
  (bind _generationvariance (`self.GenerationVariance`))
  (set `self.SinceLastGeneration` 0.0)
  (set `self.DelayBeforeNextGeneration` (+ (`self.DelayBetweenGenerations`) (`KismetMathLibrary.RandomFloatInRange` (* _generationvariance -1.0) _generationvariance))))

(fn `ShouldSpawnMeteor`
  (params (Delta :type "Float (double-precision)"))
  (returns (`Should Spawn` :type Boolean))
  (bind _output_get (set `self.SinceLastGeneration` (+ Delta (`self.SinceLastGeneration`))))
  (return (>= _output_get (`self.DelayBeforeNextGeneration`))))

(fn `SpawnMeteor`
  (bind (_min _max) (break `Box` (`self.SourceBox`)))
  (bind (_min_2 _max_2) (break `Box` (`self.DestinationBox`)))
  (bind _returnvalue (`|SpawnActorFromClass` "/Game/RocketDefender/AI/BP_Meteor.BP_Meteor_C" (`KismetMathLibrary.Conv_VectorToTransform` (`KismetMathLibrary.RandomPointInBoundingBox` _min (- _max _min))) "Undefined" "OverrideRootScale" null null))
  (set `/Game/RocketDefender/AI/BP_Meteor.Destination` (`KismetMathLibrary.RandomPointInBoundingBox` _min_2 (- _max_2 _min_2)) _returnvalue))

(fn `UserConstructionScript`)