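; BP_Meteor is a Rocket Defender meteor that travels to a target point and deals damage when it arrives.
; On BeginPlay it stores its origin and plays a timeline that lerps its location to Destination, moving without sweep.
; When the timeline finishes, it casts the game mode to GM_RocketDefense, applies a small random amount of damage through it, then destroys itself.
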(event `self.ReceiveBeginPlay`
  (set `self.Origin` (`self.K2_GetActorLocation`))
  (bind (_direction _newlocation) (`Timeline|Timeline_0` :!via `PlayFromStart`)
    (:`Update`
      (`self.K2_SetActorLocation` (`KismetMathLibrary.VLerp` (`self.Origin`) (`self.Destination`) _newlocation)))
    (:`Finished`
      (bind _asgm_rocket_defense (cast `/Game/RocketDefender/Blueprints/GM_RocketDefense` (`GameplayStatics.GetGameMode`)))
      (`/Game/RocketDefender/Blueprints/GM_RocketDefense.TakeDamage` _asgm_rocket_defense (`KismetMathLibrary.RandomIntegerInRange` 5 10))
      (`self.K2_DestroyActor`))))

(fn `UserConstructionScript`)